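; Game mode for a team-based hide-and-seek style match that spawns players on request.
; RequestSpawn switches on the team, spawning a CharacterHunter for Team A or a CharacterHider for Team B at a randomly chosen PlayerStart.
; The spawned pawn receives its team, is possessed by the requesting controller and is added to the MainGameState's Players array.
; Both teams draw from the same unfiltered pool of PlayerStarts.
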(event `RequestSpawn`
  (params (Team :type "/Game/Blueprints/TheTeam Enum" :default "NewEnumerator0") (Controller :type "Controller Object Reference"))
  (bind _players (`/Game/Blueprints/MainGameState.Players` (cast `/Game/Blueprints/MainGameState` (`GameplayStatics.GetGameState`) :!pure true)))
  (switch `/Game/Blueprints/TheTeam` Team
    (:`NewEnumerator1`
      (bind _outactors (`GameplayStatics.GetAllActorsOfClass` "/Script/Engine.PlayerStart"))
      (bind _returnvalue (`|SpawnActorFromClass` "/Game/Characters/CharacterHunter.CharacterHunter_C" (`self.GetTransform` (`|GetArrayItem` _outactors (`KismetMathLibrary.RandomInteger` (`KismetArrayLibrary.Array_Length` _outactors)))) "AdjustIfPossibleButAlwaysSpawn" "OverrideRootScale" null Team null))
      (`Controller.Possess` Controller _returnvalue)
      (`KismetArrayLibrary.Array_AddUnique` _players _returnvalue))
    (:`NewEnumerator2`
      (bind _outactors_2 (`GameplayStatics.GetAllActorsOfClass` "/Script/Engine.PlayerStart"))
      (bind _returnvalue_2 (`|SpawnActorFromClass` "/Game/Characters/CharacterHider.CharacterHider_C" (`self.GetTransform` (`|GetArrayItem` _outactors_2 (`KismetMathLibrary.RandomInteger` (`KismetArrayLibrary.Array_Length` _outactors_2)))) "AdjustIfPossibleButAlwaysSpawn" "OverrideRootScale" null Team null))
      (`Controller.Possess` Controller _returnvalue_2)
      (`KismetArrayLibrary.Array_AddUnique` _players _returnvalue_2))))

(fn `UserConstructionScript`)
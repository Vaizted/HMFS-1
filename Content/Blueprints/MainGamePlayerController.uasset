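; Player controller that handles a player's entry into a team-based game, from a starting view through team selection to spawning.
; On BeginPlay, the authority possesses the first StartingView actor found in the level, while the local controller opens the TeamSelection widget and shows the mouse cursor.
; The TeamSelected event passes the chosen team and this controller to MainGameMode's RequestSpawn.
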(event `self.ReceiveBeginPlay`
  (`|ExecutionSequence`
    (:`then_0`
      (`/Engine/EditorBlueprintResources/ActorMacros.Switch Has Authority`
        (:`Authority`
          (bind _outactors (`GameplayStatics.GetAllActorsOfClass` "/Game/Blueprints/StartingView.StartingView_C"))
          (`self.Possess` (`|GetArrayItem` _outactors)))))
    (:`then_1`
      (if (`self.IsLocalController`)
        (bind _returnvalue (`|CreateWidget` "/Game/UMG/TeamSelection.TeamSelection_C"))
        (`UserWidget.AddToViewport` _returnvalue 0)
        (set `self.bShowMouseCursor` true)))))

(event `TeamSelected`
  (params (Team :type "/Game/Blueprints/TheTeam Enum" :default "NewEnumerator0"))
  (`/Game/Blueprints/MainGameMode.RequestSpawn` (cast `/Game/Blueprints/MainGameMode` (`GameplayStatics.GetGameMode`) :!pure true) Team self))

(fn `UserConstructionScript`)